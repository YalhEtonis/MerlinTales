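; BP_PotionPush is a thrown potion projectile that knocks pawns back and damages them.
; Half a second after BeginPlay it enables blocking collision, becomes active and applies its Velocity to projectile movement.
; Its first hit marks a bounce; later hits, once active, explode it with sound and AI noise.
; Every hit also sphere-traces for one pawn, launching enemies or players along a fixed world vector, with debug drawing left on.
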(event OnComponentHit(Potion)
  (params (HitComponent :type Primitive%20Component%20Object%20Reference) (OtherActor :type Actor%20Object%20Reference) (OtherComp :type Primitive%20Component%20Object%20Reference) (NormalImpulse :type Vector :default "0, 0, 0") (Hit :type Hit%20Result%20Structure%20%28by%20ref%29))
  (bind _returnvalue (Transformation|GetActorLocation))
  (Utilities|FlowControl|Sequence
    (:then_0
      (if (Variables|Default|GetBounced)
        (if (Variables|Default|GetActive)
          (Effects|SpawnEmitteratLocation "/Game/StarterContent/Particles/P_Explosion.P_Explosion" _returnvalue)
          (Class|Actor|MakeNoise 1e+06 0 _returnvalue 0.0 "BottleBreak")
          (Audio|PlaySoundatLocation "/Game/Sound/WAV/Abstract_Pop_03.Abstract_Pop_03" _returnvalue "0, 0, 0" 1.0 1.0 0.0 0 0 0 0)
          (Actor|DestroyActor))
        (else
          (Variables|Default|SetBounced true))))
    (:then_1
      (bind (_outhit _returnvalue_2) (Collision|SphereTraceForObjects _returnvalue _returnvalue 2.5e+02 (Utilities|Array|MakeArray "ObjectTypeQuery3") false 0 "ForDuration"))
      (if _returnvalue_2
        (Utilities|FlowControl|Sequence
          (:then_0
            (bind _asbp_enemy (Utilities|Casting|CastToBP_Enemy (.HitActor (Collision|BreakHitResult _outhit))))
            (Character|LaunchCharacter _asbp_enemy (Math|Vector|MakeVector 4e+02 4e+02 2e+02) false false)
            (Game|Damage|ApplyDamage (.HitActor (Collision|BreakHitResult _outhit)) 1.0 0 0))
          (:then_1
            (bind _asbp_top_down_character (Utilities|Casting|CastToBP_TopDownCharacter (.HitActor (Collision|BreakHitResult _outhit))))
            (Character|LaunchCharacter _asbp_top_down_character (Math|Vector|MakeVector 4e+02 4e+02 2e+02) false false)
            (Game|Damage|ApplyDamage (.HitActor (Collision|BreakHitResult _outhit)) 1.0 0 0)))))))

(event EventBeginPlay
  (Utilities|FlowControl|Delay 0.5)
  (Collision|SetCollisionResponsetoAllChannels (Variables|Default|GetPotion) "ECR_Block")
  (Variables|Default|SetActive true)
  (Variables|/Script/Engine.MovementComponent|SetVelocity (Variables|Default|GetProjectileMovementPush) (Variables|Default|GetVelocity)))

(fn ConstructionScript
  (Transformation|SetWorldScale3D (Variables|Default|GetPotion) "0.250000,0.200000,0.250000"))