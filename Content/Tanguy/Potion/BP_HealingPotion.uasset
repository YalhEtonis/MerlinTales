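; Thrown healing potion bottle that bounces once and breaks on a later hit; no healing logic is present here.
; After a short BeginPlay delay it blocks all collision channels, becomes active and applies its Velocity variable to ProjectileMovement.
; The first hit only marks it as bounced.
; A later hit while active spawns an explosion and pop sound, emits a very loud "BottleBreak" noise event, then destroys the actor.
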(event OnComponentHit(Potion)
  (params (HitComponent :type Primitive%20Component%20Object%20Reference) (OtherActor :type Actor%20Object%20Reference) (OtherComp :type Primitive%20Component%20Object%20Reference) (NormalImpulse :type Vector :default "0, 0, 0") (Hit :type Hit%20Result%20Structure%20%28by%20ref%29))
  (bind _returnvalue (Transformation|GetActorLocation))
  (Utilities|FlowControl|Sequence
    (:then_0
      (if (Variables|Default|GetBounced)
        (if (Variables|Default|GetActive)
          (Effects|SpawnEmitteratLocation "/Game/StarterContent/Particles/P_Explosion.P_Explosion" _returnvalue)
          (Class|Actor|MakeNoise 1e+06 0 _returnvalue 0.0 "BottleBreak")
          (Audio|PlaySoundatLocation "/Game/Sound/WAV/Abstract_Pop_03.Abstract_Pop_03" _returnvalue "0, 0, 0" 1.0 1.0 0.0 0 0 0 0)
          (Actor|DestroyActor))
        (else
          (Variables|Default|SetBounced true))))))

(event EventBeginPlay
  (Utilities|FlowControl|Delay 0.5)
  (Collision|SetCollisionResponsetoAllChannels (Variables|Default|GetPotion) "ECR_Block")
  (Variables|Default|SetActive true)
  (Variables|/Script/Engine.MovementComponent|SetVelocity (Variables|Default|GetProjectileMovement) (Variables|Default|GetVelocity)))

(fn ConstructionScript
  (Transformation|SetWorldScale3D (Variables|Default|GetPotion) "0.250000,0.200000,0.250000"))