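; BP_IceSlide is an ice zone, filed with the potion assets, that makes the top-down player character and enemies slide while inside its sphere.
; On sphere overlap it casts to BP_TopDownCharacter and BP_Enemy, then removes ground friction and lowers walking braking deceleration on their CharacterMovement.
; On exit it writes back fixed friction and braking values rather than each character's saved originals.
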(event OnComponentBeginOverlap(Sphere)
  (params (OverlappedComponent :type Primitive%20Component%20Object%20Reference) (OtherActor :type Actor%20Object%20Reference) (OtherComp :type Primitive%20Component%20Object%20Reference) (OtherBodyIndex :type Integer) (bFromSweep :type Boolean) (SweepResult :type Hit%20Result%20Structure%20%28by%20ref%29))
  (Utilities|FlowControl|Sequence
    (:then_0
      (bind _asbp_top_down_character (Utilities|Casting|CastToBP_TopDownCharacter OtherActor))
      (Variables|/Script/Engine.CharacterMovementComponent|SetGroundFriction (Variables|/Script/Engine.Character|GetCharacterMovement _asbp_top_down_character) 0.0)
      (Variables|/Script/Engine.CharacterMovementComponent|SetBrakingDecelerationWalking (Variables|/Script/Engine.Character|GetCharacterMovement _asbp_top_down_character) 3.5e+02))
    (:then_1
      (bind _asbp_enemy (Utilities|Casting|CastToBP_Enemy OtherActor))
      (Variables|/Script/Engine.CharacterMovementComponent|SetGroundFriction (Variables|/Script/Engine.Character|GetCharacterMovement _asbp_enemy) 0.0)
      (Variables|/Script/Engine.CharacterMovementComponent|SetBrakingDecelerationWalking (Variables|/Script/Engine.Character|GetCharacterMovement _asbp_enemy) 3.5e+02))))

(event OnComponentEndOverlap(Sphere)
  (params (OverlappedComponent :type Primitive%20Component%20Object%20Reference) (OtherActor :type Actor%20Object%20Reference) (OtherComp :type Primitive%20Component%20Object%20Reference) (OtherBodyIndex :type Integer))
  (Utilities|FlowControl|Sequence
    (:then_0
      (bind _asbp_top_down_character (Utilities|Casting|CastToBP_TopDownCharacter OtherActor))
      (Variables|/Script/Engine.CharacterMovementComponent|SetGroundFriction (Variables|/Script/Engine.Character|GetCharacterMovement _asbp_top_down_character) 8.0)
      (Variables|/Script/Engine.CharacterMovementComponent|SetBrakingDecelerationWalking (Variables|/Script/Engine.Character|GetCharacterMovement _asbp_top_down_character) 1e+03))
    (:then_1
      (bind _asbp_enemy (Utilities|Casting|CastToBP_Enemy OtherActor))
      (Variables|/Script/Engine.CharacterMovementComponent|SetGroundFriction (Variables|/Script/Engine.Character|GetCharacterMovement _asbp_enemy) 8.0)
      (Variables|/Script/Engine.CharacterMovementComponent|SetBrakingDecelerationWalking (Variables|/Script/Engine.Character|GetCharacterMovement _asbp_enemy) 1e+03))))

(fn ConstructionScript)