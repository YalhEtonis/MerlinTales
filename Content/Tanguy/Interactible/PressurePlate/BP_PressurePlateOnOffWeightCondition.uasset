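; Pressure plate Blueprint that toggles a referenced door when a heavy top-down character steps on it.
; Begin overlap checks the character's IsHeavy flag, then calls Switch on the door, prints a debug message and plays the plate timeline.
; Any end overlap only reverses the timeline, leaving the door as switched.
; The lerp meant to lower the plate mesh is unwired, so the plate never moves.
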(event OnComponentBeginOverlap(Collision)
  (params (OverlappedComponent :type Primitive%20Component%20Object%20Reference) (OtherActor :type Actor%20Object%20Reference) (OtherComp :type Primitive%20Component%20Object%20Reference) (OtherBodyIndex :type Integer) (bFromSweep :type Boolean) (SweepResult :type Hit%20Result%20Structure%20%28by%20ref%29))
  (bind _asbp_top_down_character (Utilities|Casting|CastToBP_TopDownCharacter OtherActor))
  (if (Variables|/Game/TopDown/Blueprints/BP_TopDownCharacter.BP_TopDownCharacter_C|GetIsHeavy? _asbp_top_down_character)
    (Default|Switch (Variables|Default|GetDoorRef))
    (Development|PrintString "Plate press" true true "(R=1.000000,G=0.000000,B=0.186844,A=1.000000)")
    (bind _newtrack_0 (Timeline|Plate%20Timeline Play))))

(event OnComponentEndOverlap(Collision)
  (params (OverlappedComponent :type Primitive%20Component%20Object%20Reference) (OtherActor :type Actor%20Object%20Reference) (OtherComp :type Primitive%20Component%20Object%20Reference) (OtherBodyIndex :type Integer))
  (bind _newtrack_0 (Timeline|Plate%20Timeline Reverse)))

(fn ConstructionScript)