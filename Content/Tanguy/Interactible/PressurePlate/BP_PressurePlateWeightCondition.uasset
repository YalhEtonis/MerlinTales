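; Pressure plate that only a heavy BP_TopDownCharacter triggers, switching its referenced door.
; Each Tick it sphere-traces for Pawns at its collision point, with debug drawing, and checks the character's IsHeavy flag.
; A press disables Tick, calls Switch on DoorRef and plays a timeline that sinks the plate and re-enables Tick on update.
; The unpress logic is unconnected, so the plate never rises.
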(event EventTick
  (params (DeltaSeconds :type Float%20%28single-precision%29))
  (bind _collision (Variables|Default|GetCollision))
  (bind _returnvalue (Transformation|GetWorldLocation _collision))
  (bind (_outhit _returnvalue_2) (Collision|SphereTraceForObjects _returnvalue _returnvalue 1e+02 (Utilities|Array|MakeArray "ObjectTypeQuery3") false 0 "ForDuration" true "(R=1.000000,G=0.000000,B=0.000000,A=1.000000)" "(R=0.000000,G=1.000000,B=0.000000,A=1.000000)" 1e+03))
  (bind _asbp_top_down_character (Utilities|Casting|CastToBP_TopDownCharacter (.HitActor (Collision|BreakHitResult _outhit))))
  (if (Variables|/Game/TopDown/Blueprints/BP_TopDownCharacter.BP_TopDownCharacter_C|GetIsHeavy? _asbp_top_down_character)
    (Actor|Tick|SetActorTickEnabled (not _returnvalue_2))
    (Default|Switch (Variables|Default|GetDoorRef))
    (Development|PrintString "Plate press" true true "(R=1.000000,G=0.000000,B=0.186844,A=1.000000)")
    (bind _newtrack_0 (Timeline|Plate%20Timeline Play)
      (:Update
        (Transformation|SetRelativeLocation (Variables|Default|GetPlate) (Math|Vector|MakeVector 0.0 0.0 (Math|Float|Lerp 0.0 -4.5 _newtrack_0)) false false)
        (Actor|Tick|SetActorTickEnabled true)))))

(fn ConstructionScript)

(fn NewFunction
  (params (NewParam :type Boolean))
  (return NewParam))