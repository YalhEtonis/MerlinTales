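; Enemy AI character Blueprint that melee-attacks the top-down player and reacts to taking damage.
; AttackPlayer runs a short forward sphere trace for pawns, then plays an attack montage and applies damage to a hit BP_TopDownCharacter.
; Taking damage sets a hit flag and the TakeDamage blackboard key, calls Reset and reports an AI damage sense event.
; PlayMontageFalling issues an AI move, then chains fall and get-up montages.
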(event Custom|Play%20Montage%20Falling
  (bind _mesh (Variables|Character|GetMesh))
  (AI|AIMoveTo 0 (Transformation|GetActorLocation (Variables|Default|GetBp_enemy)) 0 5.0 false
    (:then
      (Animation|Montage|PlayMontage _mesh "/Game/Characters/Mannequins/Animations/Retageted/MMmontage_Fall.MMmontage_Fall"
        (:OnCompleted
          (Animation|Montage|PlayMontage _mesh "/Game/Characters/Mannequins/Animations/Retageted/MMmontage_GetUp.MMmontage_GetUp"))))))

(event Custom|AttackPlayer
  (bind _returnvalue (Transformation|GetActorLocation))
  ;[1 1 1] Attack Player and make damage
  (bind (_outhit _returnvalue_2) (Collision|SphereTraceForObjects _returnvalue (+ _returnvalue (* (Math|Vector|GetForwardVector (Transformation|GetActorRotation)) 5e+01)) 5e+01 (Utilities|Array|MakeArray "ObjectTypeQuery3") false 0 "None"))
  (if _returnvalue_2
    (Utilities|Casting|CastToBP_TopDownCharacter (.HitActor (Collision|BreakHitResult _outhit)))
    (Animation|PlayAnimMontage "/Game/Characters/Mannequins/Animations/Manny/MMmontage_AttackTemp.MMmontage_AttackTemp" 1.0 "None")
    (Game|Damage|ApplyDamage (.HitActor (Collision|BreakHitResult _outhit)) 1.0 0 (.HitActor (Collision|BreakHitResult _outhit)))
    (Development|PrintString "make damage ")))

(event Game|Damage|EventAnyDamage
  (params (Damage :type Float%20%28single-precision%29) (DamageType :type Damage%20Type%20Object%20Reference) (InstigatedBy :type Controller%20Object%20Reference) (DamageCauser :type Actor%20Object%20Reference))
  (bind _returnvalue (Utilities|Name|MakeLiteralName "TakeDamage"))
  ;[1 1 1] indique qu'il recois un dommage
  (Variables|Default|SetGetHit (<= Damage 1.0))
  (AI|Components|Blackboard|SetValueasBool (AI|GetBlackboard 0) _returnvalue true)
  (Development|PrintString "Stun")
  (Class|TypedElementListLibrary|Reset)
  (Class|AISenseDamage|ReportDamageEvent 0 0 Damage "0, 0, 0" "0, 0, 0" _returnvalue))

(event Collision|EventActorBeginOverlap
  (params (OtherActor :type Actor%20Object%20Reference)))

(event EventTick
  (params (DeltaSeconds :type Float%20%28single-precision%29)))

(fn ConstructionScript)

(fn OnRepTakeDamage)