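; Base enemy Blueprint that wanders the level and chases pawns it sees.
; From BeginPlay it moves to a random reachable point within a radius of itself, repeating each time a move succeeds.
; When PawnSensing spots a pawn it moves toward that actor, while a retriggerable delay restarts wandering shortly after sightings stop.
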(event OnSeePawn(PawnSensing)
  (params (Pawn :type Pawn%20Object%20Reference))
  (Utilities|FlowControl|Sequence
    (:then_0
      (AI|AIMoveTo self "0, 0, 0" Pawn 5.0 false))
    (:then_1
      (Utilities|FlowControl|RetriggerableDelay 1.0)
      (CallFunction|Walk))))

(event Custom|Walk
  (AI|AIMoveTo self (.RandomLocation (AI|Navigation|GetRandomReachablePointinRadius (Transformation|GetActorLocation) 5e+02 0 0)) 0 5.0 false
    (:OnSuccess
      (CallFunction|Walk))))

(event EventBeginPlay
  (CallFunction|Walk))

(fn ConstructionScript)